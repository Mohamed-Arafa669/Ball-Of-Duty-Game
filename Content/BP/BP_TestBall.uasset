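; BP_TestBall is a ball actor whose static mesh can be pushed with physics impulses and then settled back onto the actor.
; BallMechs pushes it away from an origin point, while ApplyForceWD pushes along a given direction, both enabling simulation and applying mass-independent velocity changes.
; AttachtoActor stops simulation, moves the actor to the mesh's location and reattaches the mesh to the root, resyncing the two.
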(event EventBeginPlay)

(event Collision|EventActorBeginOverlap
  (params (OtherActor :type Actor%20Object%20Reference)))

(event EventTick
  (params (DeltaSeconds :type Float%20%28single-precision%29)))

(event EventBallMechs
  (params (Forcing%20Origin :type Vector :default "0, 0, 0") (power :type Float%20%28single-precision%29))
  (bind _staticmesh (Variables|Default|GetStaticMesh))
  (Physics|SetSimulatePhysics _staticmesh true)
  (Physics|AddImpulse _staticmesh (* (Math|Vector|Normalize (- (Transformation|GetWorldLocation _staticmesh) Forcing%20Origin)) power) "None" true))

(event EventApplyForceWD
  (params (Direction :type Vector :default "0, 0, 0") (power :type Float%20%28single-precision%29))
  (bind _staticmesh (Variables|Default|GetStaticMesh))
  (Physics|SetSimulatePhysics _staticmesh true)
  (Physics|AddImpulse _staticmesh (* Direction power) "None" true))

(event EventAttachtoActor
  (bind _staticmesh (Variables|Default|GetStaticMesh))
  (if (Physics|IsSimulatingPhysics _staticmesh "None")
    (Physics|SetSimulatePhysics _staticmesh false)
    (Transformation|SetActorLocation (Transformation|GetWorldLocation _staticmesh) false false)
    (Transformation|AttachComponentToComponent (Variables|Default|GetStaticMesh) (Variables|Default|GetDefaultSceneRoot) "None" "KeepWorld" "KeepWorld" "KeepWorld" true)))

(fn ConstructionScript)