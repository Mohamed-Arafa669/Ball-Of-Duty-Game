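; Player controller with disconnected logic for spawning and possessing the character selected in the game instance.
; BeginPlay and both custom spawn events are empty, so none of this logic runs.
; The orphaned chains set game-only input, pass the selected class from NewGameInstance to the server spawn event, and spawn at a PlayerStart.
; The PlayerStart search uses a "Found" tag and stops at the first start without it.
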(event Custom|CE_SpawnCharacter)

(event Custom|SE_SpawnCharacterServer
  (params (CharacterClass :type Character%20Class%20Reference)))

(event EventTick
  (params (DeltaSeconds :type Float%20%28single-precision%29)))

(event EventBeginPlay)

(fn ConstructionScript)